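; Stats component for BP_Character that tracks health and mana and caches its owning character on BeginPlay.
; Damage, healing and max-health increases update CurrentHealth and push the ratio to the HUD health bar, with damage reporting death at zero.
; Mana spending returns whether mana has fallen to a low threshold, while regeneration adds a fixed step up to a hardcoded cap.
; Mana changes do not update the HUD.
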(event `self.ReceiveBeginPlay`
  (bind _asbp_character (cast `/Game/BP_Character` (`self.GetOwner`)))
  (set `self.Player BP` _asbp_character))

(fn `Decrease Health`
  (params (Damage :type "Float (double-precision)"))
  (returns (`Is Player Dead` :type Boolean))
  (bind _output_get (set `self.CurrentHealth` (- (`self.CurrentHealth`) Damage)))
  (`ProgressBar.SetPercent` (`/Game/WBP_HUD.HealthBar` (`/Game/BP_Character.HUD Widget` (`self.Player BP`))) (/ _output_get (`self.MaxHealth`)))
  (if (<= (`self.CurrentHealth`) 0.0)
    (return true)
    (else
      (return false))))

(fn `Decrease Mana`
  (params (ManaCost :type "Float (double-precision)"))
  (returns (`Mana Insufficient` :type Boolean))
  (set `self.Current Mana` (- (`self.Current Mana`) ManaCost))
  (if (<= (`self.Current Mana`) 10.0)
    (return true)
    (else
      (return false))))

(fn `Heal`
  (params (`Heal Amount` :type "Float (double-precision)"))
  (set `self.CurrentHealth` (+ (`self.CurrentHealth`) `Heal Amount`))
  (if (>= (`self.CurrentHealth`) (`self.MaxHealth`))
    (set `self.CurrentHealth` (`self.MaxHealth`)))
  (`ProgressBar.SetPercent` (`/Game/WBP_HUD.HealthBar` (`/Game/BP_Character.HUD Widget` (`self.Player BP`))) (/ (`self.CurrentHealth`) (`self.MaxHealth`))))

(fn `Increase Mana`
  (if (<= (`self.Current Mana`) 65.0)
    (set `self.Current Mana` (+ (`self.Current Mana`) 5.0))
    (else
      (set `self.Current Mana` 70.0))))

(fn `Increase Max Health`
  (params (HealthAdded :type "Float (double-precision)"))
  (bind _output_get (set `self.MaxHealth` (+ (`self.MaxHealth`) HealthAdded)))
  (bind _output_get_2 (set `self.CurrentHealth` _output_get))
  (`ProgressBar.SetPercent` (`/Game/WBP_HUD.HealthBar` (`/Game/BP_Character.HUD Widget` (`self.Player BP`))) (/ _output_get_2 (`self.MaxHealth`))))